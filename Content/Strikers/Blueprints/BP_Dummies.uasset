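; Patrolling dummy actor that moves its static mesh in a continuous loop along a spline.
; BeginPlay detaches the Patrol spline to keep it fixed in world space and sets a one-shot timer on Patrolling, which Tick also calls.
; Each call advances distance by PatrolSpeed, making movement frame-rate dependent, and wraps at the spline's end.
; An older target-point patrol draft remains unconnected.
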(event `self.ReceiveBeginPlay`
  (`SceneComponent.K2_DetachFromComponent` (`self.Patrol`) "KeepWorld" "KeepWorld" "KeepWorld" true)
  (`KismetSystemLibrary.K2_SetTimerDelegate` (delegate `Patrolling`) 0.5))

(event `Patrolling`
  (bind _returnvalue (`SplineComponent.GetSplineLength` (`self.Patrol`)))
  (bind _output_get (set `self.DistanceOnSpline` (+ (`self.DistanceOnSpline`) (`self.PatrolSpeed`))))
  (if (not (< _output_get _returnvalue))
    (set `self.DistanceOnSpline` (- (`self.DistanceOnSpline`) _returnvalue)))
  (bind _output_get_2 (set `self.PatrolNextLocation` (`SplineComponent.GetLocationAtDistanceAlongSpline` (`self.Patrol`) (`self.DistanceOnSpline`) "World")))
  (`SceneComponent.K2_SetWorldLocation` (`self.StaticMesh`) _output_get_2 false false))

(event `self.ReceiveTick`
  (params (DeltaSeconds :type "Float (single-precision)"))
  (`self.Patrolling`))

(fn `UserConstructionScript`)