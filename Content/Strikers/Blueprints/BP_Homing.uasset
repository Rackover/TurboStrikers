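; BP_Homing is a homing missile actor that pursues a target actor and destroys itself when its lifespan runs out.
; InitializeData copies tuning from a homing struct, sets an initial rotation, then activates the missile.
; Server-only Tick offsets it by blending forward inertia with target direction, weighted by speed and Accuracy, while accelerating toward max speed.
; Damage is stored but unused here, and Tick never updates rotation.
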(event `OnActivation`
  (set `self.IsActivated` true)
  (`KismetSystemLibrary.Delay` (`self.Lifespan`))
  (`self.K2_DestroyActor`))

(event `self.ReceiveTick`
  (params (DeltaSeconds :type "Float (single-precision)"))
  (bind _returnvalue (`self.GetActorForwardVector`))
  (if (`self.IsActivated`)
    (`/Engine/EditorBlueprintResources/ActorMacros.Switch Has Authority`
      (:`Authority`
        (set `self.TargetPosition` (`self.K2_GetActorLocation` (`self.MissileTarget`)))
        (`self.K2_AddActorLocalOffset` (+ (* _returnvalue (/ (`self.MissileSpeed`) 100.0)) (`KismetMathLibrary.VLerp` _returnvalue (* (`KismetMathLibrary.Normal` (- (`self.TargetPosition`) (`self.K2_GetActorLocation`))) (`self.MissileSpeed`)) (`KismetMathLibrary.FMax` (`KismetMathLibrary.NormalizeToRange` (/ (- (`self.MissileMaxSpeed`) (`self.MissileSpeed`)) (`self.MissileMaxSpeed`)) 0.0 1.0) (`self.Accuracy`)))))
        ;[1 1 1] Is missile fast enough?
        (if (>= (`self.MissileSpeed`) (`self.MissileMaxSpeed`))
          (set `self.MissileSpeed` (`self.MissileMaxSpeed`))
          (else
            ;[1 1 1] Accelerate the missile
            (set `self.MissileSpeed` (+ (`self.MissileSpeed`) (* (`self.AccelerationFactor`) (`GameplayStatics.GetWorldDeltaSeconds`))))))))))

(fn `InitializeData`
  (params (ActualHomingStruct :type "/Game/Strikers/Weapons/HomingWeapon Structure") (MissileTarget :type "Actor Object Reference") (MissileOwner :type "Actor Object Reference"))
  (bind (_maxspeed _damage _lockingrange _lifetime _accelerationfactor _reloadtime _accuracy) (break `/Game/Strikers/Weapons/HomingWeapon` ActualHomingStruct))
  (bind _returnvalue (`KismetMathLibrary.Conv_VectorToRotator` (`KismetMathLibrary.Normal` (- (`self.TargetPosition`) (`self.K2_GetActorLocation` (`self.MissileTarget`))))))
  (set `self.MissileOwner` MissileOwner)
  (set `self.MissileTarget` MissileTarget)
  (set `self.MissileMaxSpeed` _maxspeed)
  (set `self.Lifespan` _lifetime)
  (set `self.AccelerationFactor` _accelerationfactor)
  (set `self.Accuracy` _accuracy)
  (set `self.Damage` _damage)
  (`/Engine/EditorBlueprintResources/StandardMacros.IsValid` (`self.MissileOwner`)
    (:`Is Valid`
      (`self.K2_SetActorRotation` _returnvalue true)
      (`KismetSystemLibrary.PrintString` (`KismetStringLibrary.Concat_StrStr` "ROT : " (`KismetStringLibrary.Conv_RotatorToString` _returnvalue)) true true (struct :`R` 1.0 :`G` 0.661581 :`A` 1.0) 50.0))
    (:`Is Not Valid`
      _))
  (`self.OnActivation`))

(fn `UserConstructionScript`)