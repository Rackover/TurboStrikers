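; BP_NetworkClient handles LAN multiplayer sessions for Strikers, exposing Host, List, Join and Kill events.
; Host creates a LAN session and opens Map_Paradise as a listen server.
; List searches for LAN sessions, prints their server names and caches the results, from which Join connects to the first entry.
; Kill destroys the current session, and all operations report progress and errors only through on-screen debug prints.
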(event `Host`
  ;[0 1 0.9906] NETWORKING
  ;;[1 1 1] Host
  (`CreateSessionCallbackProxy.CreateSession` (`GameplayStatics.GetPlayerController` 0) 64 true
    (:`then`
      (`KismetSystemLibrary.PrintString` "Hosting..."))
    (:`OnSuccess`
      (`KismetSystemLibrary.PrintString` "Hosted !")
      (`GameplayStatics.OpenLevel` "Map_Paradise" true "listen"))
    (:`OnFailure`
      (`KismetSystemLibrary.PrintString` "ERROR Cannot host"))))

(event `List`
  ;[0 1 0.9906] NETWORKING
  ;;[1 1 1] List sessions
  (bind _results (`FindSessionsCallbackProxy.FindSessions` (`GameplayStatics.GetPlayerController` 0) 5 true)
    (:`then`
      (`KismetSystemLibrary.PrintString` "Listing..."))
    (:`OnSuccess`
      (`KismetSystemLibrary.PrintString` (`KismetStringLibrary.Concat_StrStr` "Found: " (`KismetStringLibrary.Conv_IntToString` (`KismetArrayLibrary.Array_Length` _results))))
      (for _array_element _results
        (`KismetSystemLibrary.PrintString` (`FindSessionsCallbackProxy.GetServerName` _array_element)))
      (`KismetSystemLibrary.PrintString` "<< PRESS J TO JOIN >>" true true (struct :`R` 1.0 :`G` 0.834771 :`A` 1.0))
      (set `self.Sessions` _results))
    (:`OnFailure`
      (`KismetSystemLibrary.PrintString` "ERROR Cannot list"))))

(event `Kill`
  ;[0 1 0.9906] NETWORKING
  ;;[1 1 1] Kill session
  (`DestroySessionCallbackProxy.DestroySession` (`GameplayStatics.GetPlayerController` 0)
    (:`then`
      (`KismetSystemLibrary.PrintString` "Killing..."))
    (:`OnSuccess`
      (`KismetSystemLibrary.PrintString` "Killed !"))
    (:`OnFailure`
      (`KismetSystemLibrary.PrintString` "ERROR Cannot kill"))))

(event `Join`
  (bind _sessions (`self.Sessions`))
  ;[0 1 0.9906] NETWORKING
  ;;[1 1 1] Join session
  (if (> (`KismetArrayLibrary.Array_Length` _sessions) 0)
    (`JoinSessionCallbackProxy.JoinSession` (`GameplayStatics.GetPlayerController` 0) (`|GetArrayItem` _sessions)
      (:`then`
        (`KismetSystemLibrary.PrintString` "Joining..."))
      (:`OnSuccess`
        (`KismetSystemLibrary.PrintString` "Joined !"))
      (:`OnFailure`
        (`KismetSystemLibrary.PrintString` "ERROR Cannot join")))
    (else
      (`KismetSystemLibrary.PrintString` "Nothing to join" true true (struct :`R` 1.0 :`B` 0.011574 :`A` 1.0)))))