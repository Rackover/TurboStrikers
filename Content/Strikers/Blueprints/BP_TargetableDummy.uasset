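; BP_TargetableDummy is a dummy actor, named as a target, whose static mesh moves along a patrol spline.
; On BeginPlay it plays the PatrolAlongSpline timeline, whose Position track is scaled by the spline length into a distance.
; Each update places the mesh at that spline point's local location plus the actor's location, so actor rotation and scale are not applied to the path.
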(event `self.ReceiveBeginPlay`
  (bind (_direction _position) (`Timeline|PatrolAlongSpline`)
    (:`Update`
      (`SceneComponent.K2_SetWorldLocation` (`self.StaticMesh`) (+ (.location (`SplineComponent.GetTransformAtDistanceAlongSpline` (`self.Patrol`) (* _position (`SplineComponent.GetSplineLength` (`self.Patrol`))) "Local" false)) (`self.K2_GetActorLocation`)) false false))))

(fn `UserConstructionScript`)