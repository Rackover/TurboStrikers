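; AI drone for Strikers that joins a random team, hunts enemies and awards a point to the Striker that destroys it.
; Server-side Tick flies toward the nearest BPI_Teamable enemy, falling back to waypoints it spawns if none exist.
; Steering lerps the forward vector toward the target before propelling.
; Distance selects homing missiles from alternating arrow components or alignment-gated spread fire from all arrows, both cooldown-limited.
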(event `self.ReceiveBeginPlay`
  (`/Engine/EditorBlueprintResources/ActorMacros.Switch Has Authority`
    (:`Authority`
      (set `self.Team` (`KismetMathLibrary.RandomInteger` 2)))))

(event `/Game/Strikers/Blueprints/BPI_Damageable.TakeDamage`
  (params (Damage :type "Float (single-precision)") (Dealer :type "Actor Object Reference"))
  (bind _output_get (set `self.Hitpoints` (- Damage (`self.Hitpoints`))))
  (if (<= _output_get 0.0)
    (bind _asbp_striker (cast `/Game/Strikers/Blueprints/FlyingCharacter/BP_Striker` Dealer))
    (`/Game/Strikers/Blueprints/FlyingCharacter/BP_Striker.IncrementScore` _asbp_striker 1)
    (`self.K2_DestroyActor`)))

(event `self.ReceiveTick`
  (params (DeltaSeconds :type "Float (single-precision)"))
  ;[1 1 1] Only works serverside
  (`/Engine/EditorBlueprintResources/ActorMacros.Switch Has Authority`
    (:`Authority`
      (bind _output (`self.FindTarget`))
      (bind _reached (`self.ReachTarget` _output))
      (bind _isenemy (`self.IsEnemy` _output)
        (:`Out`
          (if _isenemy
            (`self.AttackTarget` _output))
          (if _reached
            (bind _asbp_waypoint (cast `/Game/Strikers/Blueprints/Dummies/BP_Waypoint` _output))
            (set `self.LastWaypoint` _asbp_waypoint)))))))

(fn `AttackTarget`
  (params (Target :type "Actor Object Reference"))
  (switch `int` (`KismetMathLibrary.Conv_ByteToInt` (`self.PickWeaponDependingOnDistance` (`self.GetDistanceTo` Target)))
    (:`1`
      (`self.FireMissile` Target))
    (:`2`
      (`self.Shoot` Target))))

(fn `FindTarget`
  (returns (Output :type "Actor Object Reference"))
  (bind (_enemies _arethereanyenemies) (`self.GetEnemies`))
  (if _arethereanyenemies
    (bind _nearest (`self.GetNearestActorFromList` _enemies))
    (return _nearest)
    (else
      (bind (_waypointlist _arethereanywaypoints) (`self.GetWaypoints`))
      (if _arethereanywaypoints
        (bind _nearest_2 (`self.GetNearestActorFromList` _waypointlist))
        (return _nearest_2)
        (else
          (`self.SpawnWaypoint` (`self.K2_GetActorLocation`))
          (bind _point (`self.GetRandomPoint` (`self.WaypointGeneratorDistance`)))
          (bind _waypoint (`self.SpawnWaypoint` _point))
          (return _waypoint))))))

(fn `FireMissile`
  (params (MissileTarget :type "Actor Object Reference"))
  (locals (ThisTarget :type "Actor Object Reference"))
  (bind _output_get (set `local.ThisTarget` MissileTarget))
  (`/Engine/EditorBlueprintResources/StandardMacros.IsValid` _output_get
    (:`Is Valid`
      ;[1 1 1] Cooldown
      (if (> (`GameplayStatics.GetTimeSeconds`) (+ (`self.LastMissileShot`) (`.ReloadTime_20_146AF44043437CB2D08871B9AC6FF834` (break `/Game/Strikers/Weapons/HomingWeapon` (`self.HomingWeapon`)))))
        (bind _isa (`/Engine/EditorBlueprintResources/StandardMacros.FlipFlop`)
          (:`A`
            _)
          (:`B`
            _))
        (bind _returnvalue (`|SpawnActorFromClass` "/Game/Strikers/Blueprints/Weapons/BP_Homing_Missile.BP_Homing_Missile_C" (`SceneComponent.K2_GetComponentToWorld` (`|GetArrayItem` (`self.K2_GetComponentsByClass` "/Script/Engine.ArrowComponent") (`KismetMathLibrary.Conv_BoolToInt` _isa))) "Undefined" "OverrideRootScale" null null))
        (`/Game/Strikers/Blueprints/Weapons/BP_Homing.InitializeData` _returnvalue (`self.HomingWeapon`) (`local.ThisTarget`) self (`self.Speed`))
        (set `self.LastMissileShot` (`GameplayStatics.GetTimeSeconds`))))))

(fn `GetEnemies`
  (returns (Enemies :type "Array of Actor Object Reference") (AreThereAnyEnemies :type Boolean))
  (locals (PotentialEnemies :type "Array of Actor Object Reference") (ConfirmedEnemies :type "Array of Actor Object Reference"))
  (bind _confirmedenemies (`local.ConfirmedEnemies`))
  (bind _outactors (`GameplayStatics.GetAllActorsWithInterface` "/Game/Strikers/Blueprints/BPI_Teamable.BPI_Teamable_C"))
  (set `local.PotentialEnemies` _outactors)
  (if (> (`KismetArrayLibrary.Array_Length` _outactors) 0)
    ;[1 1 1] Keeping only enemies
    (for _array_element (`local.PotentialEnemies`)
      (bind _isenemy (`self.IsEnemy` _array_element)
        (:`Out`
          (if _isenemy
            (`KismetArrayLibrary.Array_Add` _confirmedenemies _array_element)))))
    (return _confirmedenemies (> (`KismetArrayLibrary.Array_Length` _confirmedenemies) 0))
    (else
      (return _ false))))

(fn `GetName`
  (returns (Name :type String))
  (return "UNMANNED_AIRCRAFT"))

(fn `GetNearestActorFromList`
  (params (List :type "Array of Actor Object Reference"))
  (returns (Nearest :type "Actor Object Reference"))
  (locals (EnemyCandidate :type "Actor Object Reference") (CurrentLowestDistance :type "Float (double-precision)" :default 9.999999843067494e+16))
  (for _array_element List
    (bind _returnvalue (`self.GetDistanceTo` _array_element))
    (if (< _returnvalue (`local.CurrentLowestDistance`))
      (set `local.CurrentLowestDistance` _returnvalue)
      (set `local.EnemyCandidate` _array_element)))
  (return (`local.EnemyCandidate`)))

(fn `GetRandomPoint`
  (params (Distance :type "Float (double-precision)"))
  (returns (Point :type "Vector Structure"))
  (return (+ (* (`KismetMathLibrary.MakeVector` (.x (`KismetMathLibrary.RandomUnitVector`)) (.y (`KismetMathLibrary.RandomUnitVector`)) (`KismetMathLibrary.Abs` (.z (`KismetMathLibrary.RandomUnitVector`)))) Distance) (`self.K2_GetActorLocation`))))

(fn `GetTeam`
  (returns (Team :type Integer))
  (return (`self.Team`)))

(fn `GetWaypoints`
  (returns (WaypointList :type "Array of Actor Object Reference") (AreThereAnyWaypoints :type Boolean))
  (locals (Waypoints :type "Array of Actor Object Reference"))
  (bind _outactors (`GameplayStatics.GetAllActorsOfClass` "/Game/Strikers/Blueprints/Dummies/BP_Waypoint.BP_Waypoint_C"))
  (`KismetArrayLibrary.Array_RemoveItem` _outactors (`self.LastWaypoint`))
  (bind _output_get (set `local.Waypoints` _outactors))
  (return _output_get (> (`KismetArrayLibrary.Array_Length` _outactors) 0)))

(fn `IsCurrentlyTargetable`
  (returns (IsTargetable :type Boolean))
  (return true))

(fn `OrientTowardsPosition`
  (params (Position :type "Vector Structure"))
  (`self.K2_SetActorRotation` (`KismetMathLibrary.Conv_VectorToRotator` (`KismetMathLibrary.VLerp` (`self.GetActorForwardVector`) (`KismetMathLibrary.Normal` (- Position (`self.K2_GetActorLocation`))) (`self.LookAtSpeed`)))))

(fn `Propel`
  (`self.K2_SetActorLocation` (+ (`self.K2_GetActorLocation`) (* (`self.GetActorForwardVector`) (* (`self.Speed`) (`GameplayStatics.GetWorldDeltaSeconds`))))))

(fn `ReachTarget`
  (params (Target :type "Actor Object Reference"))
  (returns (Reached :type Boolean))
  (bind _returnvalue (`self.K2_GetActorLocation` Target))
  (`self.OrientTowardsPosition` _returnvalue)
  (`self.Propel`)
  (return (`self.HasReachedPosition` _returnvalue)))

(fn `Shoot`
  (params (Enemy :type "Actor Object Reference"))
  (bind (_projectileblueprint _reloadtime _projectionspeed _spreadangle) (break `/Game/Strikers/Weapons/SpreadWeapon` (`self.SpreadWeapon`)))
  (bind (_projectileblueprint_2 _reloadtime_2 _projectionspeed_2 _spreadangle_2 _damage _lifespan) (break `/Game/Strikers/Weapons/SpreadWeapon` (`self.SpreadWeapon`)))
  (bind _returnvalue (* _spreadangle -1.0))
  (if (and (< (`KismetMathLibrary.VSize` (- (`self.GetActorForwardVector`) (`KismetMathLibrary.Normal` (- (`self.K2_GetActorLocation` Enemy) (`self.K2_GetActorLocation`))))) (`self.MinBulletAlignment`)) (> (`GameplayStatics.GetTimeSeconds`) (+ (`self.LastShot`) _reloadtime)))
    (for _array_element (`self.K2_GetComponentsByClass` "/Script/Engine.ArrowComponent")
      (bind _asarrow_component (cast `ArrowComponent` _array_element))
      (bind _returnvalue_2 (`|SpawnActorFromClass` _projectileblueprint (`KismetMathLibrary.MakeTransform` (`SceneComponent.K2_GetComponentLocation` _asarrow_component) (`SceneComponent.K2_GetComponentRotation` (`self.StaticMesh`))) "AlwaysSpawn" "OverrideRootScale" null null))
      (bind _asbp_projectile (cast `/Game/Strikers/Blueprints/Weapons/BP_Projectile` _returnvalue_2))
      (set `/Game/Strikers/Blueprints/Weapons/BP_Projectile.BaseSpeed` (+ (`self.Speed`) _projectionspeed) _asbp_projectile)
      (`self.K2_AddActorLocalRotation` _returnvalue_2 (`KismetMathLibrary.MakeRotator` 0.0 (`KismetMathLibrary.RandomFloatInRange` _returnvalue _spreadangle) (`KismetMathLibrary.RandomFloatInRange` _returnvalue _spreadangle)) false false)
      (set `self.LastShot` (`GameplayStatics.GetTimeSeconds`))
      (set `/Game/Strikers/Blueprints/Weapons/BP_Projectile.Damage` _damage _asbp_projectile)
      (set `/Game/Strikers/Blueprints/Weapons/BP_Projectile.ProjectileOwner` self _asbp_projectile)
      (set `/Game/Strikers/Blueprints/Weapons/BP_Projectile.IsActivated` true _asbp_projectile)
      (`self.SetLifeSpan` _asbp_projectile _lifespan))))

(fn `SpawnWaypoint`
  (params (Position :type "Vector Structure"))
  (returns (Waypoint :type "Actor Object Reference"))
  (bind _returnvalue (`|SpawnActorFromClass` "/Game/Strikers/Blueprints/Dummies/BP_Waypoint.BP_Waypoint_C" (`KismetMathLibrary.MakeTransform` Position) "Undefined" "OverrideRootScale" null null))
  (return _returnvalue))

(fn `UserConstructionScript`)