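; BP_PatrollingDummy is an actor that spawns a target dummy and moves it along a patrol spline.
; On BeginPlay it spawns a BP_DummyTarget at its own transform and plays the PatrolAlongSpline timeline.
; Each update scales the timeline's Position by spline length, samples the local-space point and adds the actor's location, so actor rotation and scale are not applied to the path.
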(event `self.ReceiveBeginPlay`
  (bind _returnvalue (`|SpawnActorFromClass` "/Game/Strikers/Blueprints/Dummies/BP_DummyTarget.BP_DummyTarget_C" (`self.GetTransform`) "Undefined" "OverrideRootScale" null null))
  (set `self.Dummy` _returnvalue)
  (bind (_direction _position) (`Timeline|PatrolAlongSpline`)
    (:`Update`
      (`self.K2_SetActorLocation` (`self.Dummy`) (+ (.location (`SplineComponent.GetTransformAtDistanceAlongSpline` (`self.Patrol`) (* _position (`SplineComponent.GetSplineLength` (`self.Patrol`))) "Local" false)) (`self.K2_GetActorLocation`)) false false))))

(fn `UserConstructionScript`)