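; Player flying-character Blueprint with arcade flight, guns and homing missiles, configured by a FlightModels DataTable row.
; Each tick, input feeds clamped, decaying accumulators that drive rotation, swept thrust, camera, trails and first-person HUD.
; An engine toggle ramps power against manual gravity and grants a decaying boost on start.
; Weapons use DataTable reload times, missiles target the first BP_Dummies found, and any hit teleports the player to PlayerStart.
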(event `self.ReceiveBeginPlay`
  ;[1 0.4595 0.7077] Flight Model Loading
  (set `self.PreviousTransform` (`SceneComponent.K2_GetComponentToWorld` (`self.Parent`)))
  (bind _returnvalue (`|GetDataTableRow` "/Game/Strikers/FlightModels/FlightModels.FlightModels" (`self.CurrentModelName`))
    (:`then`
      (`self.LoadFlightModel` _returnvalue)
      (bind _outactors (`GameplayStatics.GetAllActorsOfClass` "/Game/Strikers/Blueprints/BP_Dummies.BP_Dummies_C"))
      (set `self.LockedTarget` (`|GetArrayItem` _outactors))
      (set `self.MissileBlueprint` "/Game/Strikers/Blueprints/BP_Homing_Missile.BP_Homing_Missile_C"))))

(event `self.ReceiveHit`
  (params (MyComp :type "PrimitiveComponent Object Reference") (Other :type "Actor Object Reference") (OtherComp :type "PrimitiveComponent Object Reference") (bSelfMoved :type Boolean) (HitLocation :type "Vector Structure") (HitNormal :type "Vector Structure") (NormalImpulse :type "Vector Structure") (Hit :type "HitResult Structure (by ref)"))
  (bind _parent (`self.Parent`))
  ;[1 1 1] If the player hits the ground, bring her back to player start
  (bind _outactors (`GameplayStatics.GetAllActorsOfClass` "/Script/Engine.PlayerStart"))
  (`self.K2_SetActorTransform` (`self.GetTransform` (`|GetArrayItem` _outactors)) false true)
  (`PrimitiveComponent.SetPhysicsLinearVelocity` _parent (0.0 0.0 0.0) false "None")
  (`PrimitiveComponent.SetPhysicsAngularVelocityInDegrees` _parent (0.0 0.0 0.0) false "None"))

(event `self.ReceiveTick`
  (params (DeltaSeconds :type "Float (single-precision)"))
  (bind (_returnvalue_roll _returnvalue_pitch) (`KismetMathLibrary.BreakRotator` (`self.K2_GetActorRotation`)))
  (bind (_returnvalue_roll_2 _returnvalue_pitch_2 _returnvalue_yaw) (`KismetMathLibrary.BreakRotator` (`self.K2_GetActorRotation`)))
  (bind _hud (`self.HUD`))
  ;[1 0.7143 0.3672] INPUT
  (set `self.DeltaTime` DeltaSeconds)
  (if (`self.IsEngineRunning`)
    (`self.AccumulateForwardInput`))
  (`self.AccumulateRollPitchYaw`)
  ;[1 0 0] Effective movement
  (`self.UpdateEngineAccumulator`)
  (set `self.PreviousTransform` (`SceneComponent.K2_GetComponentToWorld` (`self.Parent`)))
  (`self.RotateFromAccumulators`)
  (`self.ThrustFromAccumulators`)
  ;;[1 1 1] Gravity
  (`self.ApplyGravity`)
  ;[1 1 1] Shoot
  (if (`self.IsShooting`)
    (`self.Shoot`))
  ;[1 1 1] LaunchMissile
  (if (`self.isLaunchingMissile`)
    (`self.LaunchMissile`))
  ;[1 1 1] Camera
  (`self.UpdateCameraFromThrust`)
  (`self.UpdateCameraFromAccumulators`)
  ;[1 1 1] FX
  (`self.UpdateTrailFX`)
  ;[1 1 1] Variable decay
  (`self.DecayRollPitchYaw`)
  (`self.DecayThrust`)
  (`self.DecayBoost`)
  ;[0.461 0.5606 1] HUD
  (if (`self.IsFirstPerson`)
    (`Widget.SetVisibility` _hud "Visible")
    ;;[1 1 1] Virtual horizon
    (bind _asw_hud_parent (cast `/Game/Strikers/Widgets/W_HUD_Parent` _hud))
    (`Widget.SetRenderTransform` (`/Game/Strikers/Widgets/W_HUD_Parent.VirtualHorizon` _asw_hud_parent) (make `WidgetTransform` (`KismetMathLibrary.MakeVector2D` 0.0 (* _returnvalue_pitch (`self.VirtualHorizonVerticalAmplitude`))) (1.0 1.0) (0.0 0.0) (- 0.0 _returnvalue_roll)))
    ;;[1 1 1] Engine ON/OFF
    (set `/Game/Strikers/Widgets/W_HUD_Parent.EngineState` (`self.IsEngineRunning`) _asw_hud_parent)
    ;;[1 1 1] Speedometer
    (set `/Game/Strikers/Widgets/W_HUD_Parent.Gas` (`self.GasAccumulator`) _asw_hud_parent)
    ;;[1 1 1] Sight
    (bind _forwardvectorlength (`self.GetForwardSpeed`))
    (bind _crosshaircontainer (`/Game/Strikers/Widgets/W_HUD_Parent.CrosshairContainer` _asw_hud_parent))
    (bind _returnvalue (`PanelWidget.GetChildrenCount` _crosshaircontainer))
    (for _index (range _returnvalue)
      (bind _returnvalue_2 (`PanelWidget.GetChildAt` _crosshaircontainer _index))
      (bind _returnvalue_3 (/ (`KismetMathLibrary.Conv_IntToDouble` (+ _index 1)) (`KismetMathLibrary.Conv_IntToDouble` _returnvalue)))
      (bind _returnvalue_4 (/ 0.5 _returnvalue_3))
      (`Widget.SetRenderScale` _returnvalue_2 (`KismetMathLibrary.MakeVector2D` _returnvalue_4 _returnvalue_4))
      (bind _returnvalue_5 (* _forwardvectorlength (`self.CollimatorAmplitude`)))
      (`Widget.SetRenderTranslation` _returnvalue_2 (`KismetMathLibrary.MakeVector2D` (* _returnvalue_3 (* -5.0 (`self.YawDragAccumulator`) _returnvalue_5)) (* _returnvalue_3 (* 1.0 (`self.PitchDragAccumulator`) _returnvalue_5)))))
    ;;[1 1 1] Compass
    (`Widget.SetRenderTranslation` (`/Game/Strikers/Widgets/W_HUD_Parent.CompassContainer` _asw_hud_parent) (`KismetMathLibrary.MakeVector2D` (* (`self.CompassMax`) (/ _returnvalue_yaw -180.0))))
    (else
      (`Widget.SetVisibility` _hud "Hidden"))))

(event `InputAction|FireGun`
  (params (Key :type "Key Structure"))
  ;[1 0.7143 0.3672] INPUT
  ;;[1 1 1] Shoot
  (:`Pressed`
    (set `self.IsShooting` true))
  (:`Released`
    (set `self.IsShooting` false)))

(event `InputAction|SwitchCamera`
  (params (Key :type "Key Structure"))
  ;[1 0.7143 0.3672] INPUT
  ;;[1 1 1] Camera
  (:`Pressed`
    (`self.SwitchCamera`)))

(event `InputAction|ToggleEngine`
  (params (Key :type "Key Structure"))
  ;[1 0.7143 0.3672] INPUT
  ;;[1 1 1] Engine toggle
  (:`Pressed`
    (if (not (`self.IsRestartingEngine`))
      (if (`self.IsEngineRunning`)
        (`self.EngineStops`)
        (else
          (`self.EngineStarts`))))))

(event `EngineStarts`
  ;[1 1 1] Engine starts - boost
  (set `self.IsEngineRunning` true)
  (`self.Boost`))

(event `InputAction|LaunchMissile`
  (params (Key :type "Key Structure"))
  ;[1 0.7143 0.3672] INPUT
  ;;[1 1 1] Launch Missile
  (:`Pressed`
    (set `self.isLaunchingMissile` true))
  (:`Released`
    (set `self.isLaunchingMissile` false)))

(event `EngineStops`
  ;[1 1 1] Engine stops
  (set `self.IsEngineRunning` false))

(fn `AccumulateForwardInput`
  (set `self.GasAccumulator` (`KismetMathLibrary.FClamp` (+ (* (`self.GetInputAxisValue`) (`.GasSensibility_34_0C69B47644331AF2E68E078131727D7F` (break `/Game/Strikers/FlightModels/FlightModel` (`self.FlightModel`))) (`self.DeltaTime`)) (`self.GasAccumulator`)) -1.0)))

(fn `AccumulateRollPitchYaw`
  (bind (_basethrust _thrust _forwardthrustmultiplier _mesh _rotationamplitude) (break `/Game/Strikers/FlightModels/FlightModel` (`self.FlightModel`)))
  (bind (_returnvalue_x _returnvalue_y _returnvalue_z) (`KismetMathLibrary.BreakVector` (* (* (`.RotationSensivity_52_8083C53746CD7D91FC3A2DA7986AD072` (break `/Game/Strikers/FlightModels/FlightModel` (`self.FlightModel`))) (`KismetMathLibrary.MakeVector` (`self.GetInputAxisValue`) (`self.GetInputAxisValue`) (`self.GetInputAxisValue`))) (`self.EngineAccumulator`))))
  (set `self.RollDragAccumulator` (`KismetMathLibrary.FClamp` (+ _returnvalue_x (`self.RollDragAccumulator`)) (* (.x _rotationamplitude) -1.0) (.x _rotationamplitude)))
  (set `self.PitchDragAccumulator` (`KismetMathLibrary.FClamp` (+ _returnvalue_y (`self.PitchDragAccumulator`)) (* (.y _rotationamplitude) -1.0) (.y _rotationamplitude)))
  (set `self.YawDragAccumulator` (`KismetMathLibrary.FClamp` (+ _returnvalue_z (`self.YawDragAccumulator`)) (* (.z _rotationamplitude) -1.0) (.z _rotationamplitude))))

(fn `ApplyGravity`
  (`self.K2_AddActorWorldOffset` (`KismetMathLibrary.MakeVector` 0.0 0.0 (* (* (`self.GravityForce`) (- 1.0 (`self.EngineAccumulator`))) -1.0))))

(fn `Boost`
  (set `self.BoostTimeRemaining` (`.BoostDuration_51_C40E52F74F715601E7BBA7AB2861FDC3` (break `/Game/Strikers/FlightModels/FlightModel` (`self.FlightModel`)))))

(fn `DecayBoost`
  (bind _boosttimeremaining (`self.BoostTimeRemaining`))
  (if (> _boosttimeremaining 0.0)
    (set `self.BoostTimeRemaining` (- _boosttimeremaining (`self.DeltaTime`)))))

(fn `DecayRollPitchYaw`
  (bind (_basethrust _thrust _forwardthrustmultiplier _mesh _rotationamplitude _rotationsensivity _stabilizationspeed) (break `/Game/Strikers/FlightModels/FlightModel` (`self.FlightModel`)))
  (set `self.YawDragAccumulator` (/ (`self.YawDragAccumulator`) _stabilizationspeed))
  (set `self.PitchDragAccumulator` (/ (`self.PitchDragAccumulator`) _stabilizationspeed))
  (set `self.RollDragAccumulator` (/ (`self.RollDragAccumulator`) _stabilizationspeed)))

(fn `DecayThrust`
  (set `self.GasAccumulator` (/ (`self.GasAccumulator`) (`.StabilizationSpeed_28_548805114F8D044033BF0180DB720AC9` (break `/Game/Strikers/FlightModels/FlightModel` (`self.FlightModel`))))))

(fn `GetForwardSpeed`
  (returns (ForwardVectorLength :type "Float (double-precision)"))
  (bind _angularspeed (`self.GetLocalAngularSpeed`))
  (return (.x _angularspeed)))

(fn `GetLocalAngularSpeed`
  (returns (AngularSpeed :type "Vector Structure"))
  (bind _previoustransform_location (`KismetMathLibrary.BreakTransform` (`self.PreviousTransform`)))
  (bind _returnvalue (`SceneComponent.K2_GetComponentToWorld` (`self.Parent`)))
  (return (`KismetMathLibrary.InverseTransformDirection` _returnvalue (- (.location _returnvalue) _previoustransform_location))))

(fn `LaunchMissile`
  (bind _returnvalue (`|GetDataTableRow` "/Game/Strikers/Weapons/HomingWeapons.HomingWeapons" (`.HomingWeapon_56_E4E04EE84527073AD9C43F80C072DE24` (break `/Game/Strikers/FlightModels/FlightModel` (`self.FlightModel`))))
    (:`then`
      (bind (_ishoming _maxspeed _damage _lockingrange _lifetime _accelerationfactor _reloadtime) (break `/Game/Strikers/Weapons/HomingWeapon` _returnvalue))
      (if (> (`GameplayStatics.GetTimeSeconds`) (+ (`self.LastLaunch`) _reloadtime))
        (`KismetSystemLibrary.PrintString` "Spawning Missile")
        (bind _returnvalue_2 (`|SpawnActorFromClass` (`self.MissileBlueprint`) (`KismetMathLibrary.MakeTransform` (+ (.location (`self.GetTransform`)) (0.0 0.0 -200.0))) "Undefined" "OverrideRootScale" null null))
        (`KismetSystemLibrary.PrintString` " Missile Spawned")
        (if _ishoming
          (bind _asbp_homing (cast `/Game/Strikers/Blueprints/BP_Homing` _returnvalue_2))
          (`/Game/Strikers/Blueprints/BP_Homing.InitializeData` _asbp_homing _returnvalue (`self.LockedTarget`))
          (bind _forwardvectorlength (`self.GetForwardSpeed`))
          (set `/Game/Strikers/Blueprints/BP_Homing.MissileSpeed` _forwardvectorlength _asbp_homing)
          (set `self.LastLaunch` (`GameplayStatics.GetTimeSeconds`)))))
    (:`RowNotFound`
      (`KismetSystemLibrary.PrintString` "Row not found"))))

(fn `LoadFlightModel`
  (params (FlightModel :type "/Game/Strikers/FlightModels/FlightModel Structure"))
  (bind (_basethrust _thrust _forwardthrustmultiplier _mesh _rotationamplitude _rotationsensivity _stabilizationspeed _interface) (break `/Game/Strikers/FlightModels/FlightModel` FlightModel))
  (`StaticMeshComponent.SetStaticMesh` (`self.FlyingMan`) _mesh)
  (bind _returnvalue (`|CreateWidget` _interface))
  (bind _output_get (set `self.HUD` _returnvalue))
  (`WidgetComponent.SetWidget` (`self.Widget`) _output_get)
  (set `self.FlightModel` FlightModel))

(fn `RotateFromAccumulators`
  (`SceneComponent.K2_AddLocalRotation` (`self.Parent`) (`KismetMathLibrary.MakeRotator` (`self.RollDragAccumulator`) (`self.PitchDragAccumulator`) (`self.YawDragAccumulator`)) false false))

(fn `Shoot`
  (bind _returnvalue (`|GetDataTableRow` "/Game/Strikers/Weapons/SpreadWeapons.SpreadWeapons" (`.SpreadWeapon_53_8DCFFB4B45AC0CE5CA10E2A06C2D1182` (break `/Game/Strikers/FlightModels/FlightModel` (`self.FlightModel`))))
    (:`then`
      (bind (_projectileblueprint _reloadtime _projectionspeed _spreadangle) (break `/Game/Strikers/Weapons/SpreadWeapon` _returnvalue))
      (if (> (`GameplayStatics.GetTimeSeconds`) (+ (`self.LastShot`) _reloadtime))
        (for _array_element (`self.K2_GetComponentsByClass` "/Script/Engine.ArrowComponent")
          (bind _asarrow_component (cast `ArrowComponent` _array_element))
          (bind _returnvalue_2 (`|SpawnActorFromClass` _projectileblueprint (`SceneComponent.K2_GetComponentToWorld` _asarrow_component) "Undefined" "OverrideRootScale" null null))
          (bind _asbp_projectile (cast `/Game/Strikers/Blueprints/BP_Projectile` _returnvalue_2))
          (bind _forwardvectorlength (`self.GetForwardSpeed`))
          (set `/Game/Strikers/Blueprints/BP_Projectile.BaseSpeed` (+ _forwardvectorlength _projectionspeed) _asbp_projectile)
          (bind _returnvalue_3 (* _spreadangle -1.0))
          (`self.K2_AddActorLocalRotation` _returnvalue_2 (`KismetMathLibrary.MakeRotator` 0.0 (`KismetMathLibrary.RandomFloatInRange` _returnvalue_3 _spreadangle) (`KismetMathLibrary.RandomFloatInRange` _returnvalue_3 _spreadangle)) false false)
          (set `self.LastShot` (`GameplayStatics.GetTimeSeconds`)))))))

(fn `SwitchCamera`
  (`ActorComponent.SetActive` (`self.FirstPersonCamera`) (not (`self.IsFirstPerson`)) false)
  (`ActorComponent.SetActive` (`self.ThirdPersonCamera`) (`self.IsFirstPerson`) false)
  (set `self.IsFirstPerson` (not (`self.IsFirstPerson`))))

(fn `ThrustFromAccumulators`
  (bind _parent (`self.Parent`))
  (bind _gasaccumulator (`self.GasAccumulator`))
  (bind _flightmodel (`self.FlightModel`))
  (bind (_basethrust _thrust _forwardthrustmultiplier _mesh _rotationamplitude _rotationsensivity _stabilizationspeed _interface _gassensibility _spreadweapon _homingweapon _enginereactivity _boostpower _boostduration) (break `/Game/Strikers/FlightModels/FlightModel` _flightmodel))
  (bind (_basethrust_2 _thrust_2 _forwardthrustmultiplier_2) (break `/Game/Strikers/FlightModels/FlightModel` _flightmodel))
  (`SceneComponent.K2_AddWorldOffset` _parent (* (`SceneComponent.GetForwardVector` _parent) (* (+ (* (+ (`self.EngineAccumulator`) (* _boostpower (/ (`self.BoostTimeRemaining`) _boostduration))) _basethrust_2) (* _thrust_2 _gasaccumulator) (* _forwardthrustmultiplier_2 (`KismetMathLibrary.FMax` _gasaccumulator))) (`GameplayStatics.GetWorldDeltaSeconds`))) true false))

(fn `UpdateCameraFromAccumulators`
  (bind _camerarotationamplitude (`self.CameraRotationAmplitude`))
  (bind _camerarotationamplitude_2 (`self.CameraRotationAmplitude`))
  (bind _springarm (`self.SpringArm`))
  (`SceneComponent.K2_SetRelativeRotation` _springarm (`KismetMathLibrary.MakeRotator` 0.0 (* (`self.PitchDragAccumulator`) _camerarotationamplitude) (* (* _camerarotationamplitude (`self.YawDragAccumulator`)) -1.0)) false false)
  (`SceneComponent.K2_SetRelativeLocation` _springarm (`KismetMathLibrary.MakeVector` 0.0 (* _camerarotationamplitude_2 (`self.YawDragAccumulator`)) (* (`self.PitchDragAccumulator`) _camerarotationamplitude_2)) false false))

(fn `UpdateCameraFromThrust`
  ;[1 1 1] FOV
  (`CameraComponent.SetFieldOfView` (`self.ThirdPersonCamera`) (+ (`self.BaseFOV`) (* (`KismetMathLibrary.FMax` (`self.GasAccumulator`)) (`self.AdditionalFOV`)))))

(fn `UpdateEngineAccumulator`
  (bind _returnvalue (* (`self.DeltaTime`) (`.EngineReactivity_46_91CD54584D1915829486B7A056FEDF31` (break `/Game/Strikers/FlightModels/FlightModel` (`self.FlightModel`)))))
  (if (`self.IsEngineRunning`)
    (set `self.EngineAccumulator` (`KismetMathLibrary.FClamp` (+ (`self.EngineAccumulator`) _returnvalue)))
    (else
      (set `self.EngineAccumulator` (`KismetMathLibrary.FClamp` (- (`self.EngineAccumulator`) _returnvalue))))))

(fn `UpdateTrailFX`
  (bind _forwardvectorlength (`self.GetForwardSpeed`))
  (bind _returnvalue (* (/ _forwardvectorlength (`self.TrailSpeedThreshold`)) (+ (`self.GasAccumulator`) 1.0)))
  (`ParticleSystemComponent.SetFloatParameter` (`self.ParticleSystem1`) "InstanceAlphaScaleOverLife" _returnvalue)
  (`ParticleSystemComponent.SetFloatParameter` (`self.ParticleSystem`) "InstanceAlphaScaleOverLife" _returnvalue))

(fn `UserConstructionScript`)