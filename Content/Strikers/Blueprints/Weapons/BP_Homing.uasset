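; BP_Homing is a weapon missile that chases a target actor for a set lifespan, then destroys itself.
; InitializeData copies tuning from a homing struct, sets target, owner and starting speed, then activates it.
; On authority, Tick steers by lerping forward toward the target direction by Accuracy, moves without sweep and accelerates toward a speed cap.
; Damage is stored but unused here, and the initial rotation reads TargetPosition before Tick sets it.
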(event `OnActivation`
  (set `self.IsActivated` true)
  (`KismetSystemLibrary.Delay` (`self.Lifespan`))
  (`self.K2_DestroyActor`))

(event `self.ReceiveTick`
  (params (DeltaSeconds :type "Float (single-precision)"))
  (bind _returnvalue (`KismetMathLibrary.VLerp` (`self.GetActorForwardVector`) (`KismetMathLibrary.Normal` (- (`self.TargetPosition`) (`self.K2_GetActorLocation`))) (`self.Accuracy`)))
  (if (`self.IsActivated`)
    (`/Engine/EditorBlueprintResources/ActorMacros.Switch Has Authority`
      (:`Authority`
        (set `self.TargetPosition` (`self.K2_GetActorLocation` (`self.MissileTarget`)))
        (`self.K2_SetActorRotation` (`KismetMathLibrary.Conv_VectorToRotator` _returnvalue))
        (`self.K2_SetActorLocation` (+ (* (* _returnvalue (`self.MissileSpeed`)) (`GameplayStatics.GetWorldDeltaSeconds`)) (`self.K2_GetActorLocation`)))
        ;[1 1 1] Is missile fast enough?
        (if (>= (`self.MissileSpeed`) (`self.MissileMaxSpeed`))
          (set `self.MissileSpeed` (`self.MissileMaxSpeed`))
          (else
            ;[1 1 1] Accelerate the missile
            (set `self.MissileSpeed` (+ (`self.MissileSpeed`) (* (`self.AccelerationFactor`) (`GameplayStatics.GetWorldDeltaSeconds`))))))))))

(fn `InitializeData`
  (params (ActualHomingStruct :type "/Game/Strikers/Weapons/HomingWeapon Structure") (MissileTarget :type "Actor Object Reference") (MissileOwner :type "Actor Object Reference") (InitialSpeed :type "Float (double-precision)"))
  (bind (_maxspeed _damage _lockingrange _lifetime _accelerationfactor _reloadtime _accuracy) (break `/Game/Strikers/Weapons/HomingWeapon` ActualHomingStruct))
  (set `self.MissileSpeed` InitialSpeed)
  (set `self.MissileOwner` MissileOwner)
  (set `self.MissileTarget` MissileTarget)
  (set `self.MissileMaxSpeed` _maxspeed)
  (set `self.Lifespan` _lifetime)
  (set `self.AccelerationFactor` _accelerationfactor)
  (set `self.Accuracy` _accuracy)
  (set `self.Damage` _damage)
  (`/Engine/EditorBlueprintResources/StandardMacros.IsValid` (`self.MissileOwner`)
    (:`Is Valid`
      (`self.K2_SetActorRotation` (`KismetMathLibrary.Conv_VectorToRotator` (`KismetMathLibrary.Normal` (- (`self.TargetPosition`) (`self.K2_GetActorLocation` (`self.MissileTarget`))))) true))
    (:`Is Not Valid`
      _))
  (`self.OnActivation`))

(fn `UserConstructionScript`)