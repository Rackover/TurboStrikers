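; BP_Projectile is a weapon projectile that, once activated, moves itself each Tick on the authority only.
; It sweeps forward along its local X axis by delta-scaled BulletSpeed plus a per-frame BaseSpeed.
; BulletSpeed decays linearly to zero, and a downward world-space offset grows as it falls below its initial value, faking bullet drop without physics.
; The drop offset is applied per frame without delta-time scaling.
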(event `self.ReceiveBeginPlay`
  (set `self.InitialBulletSpeed` (`self.BulletSpeed`)))

(event `self.ReceiveTick`
  (params (DeltaSeconds :type "Float (single-precision)"))
  (if (`self.IsActivated`)
    (`/Engine/EditorBlueprintResources/ActorMacros.Switch Has Authority`
      (:`Authority`
        (`self.K2_AddActorLocalTransform` (`KismetMathLibrary.MakeTransform` (`KismetMathLibrary.MakeVector` (+ (* (`GameplayStatics.GetWorldDeltaSeconds`) (`self.BulletSpeed`)) (`self.BaseSpeed`)))) true)
        (`self.K2_AddActorWorldTransform` (`KismetMathLibrary.MakeTransform` (`KismetMathLibrary.MakeVector` 0.0 0.0 (* 200.0 -1.0 (- 1.0 (/ (`self.BulletSpeed`) (`self.InitialBulletSpeed`)))))) true)
        (set `self.BulletSpeed` (`KismetMathLibrary.FMax` (- (`self.BulletSpeed`) (* (`self.BulletDecaySpeed`) (`GameplayStatics.GetWorldDeltaSeconds`)))))))))

(fn `UserConstructionScript`)