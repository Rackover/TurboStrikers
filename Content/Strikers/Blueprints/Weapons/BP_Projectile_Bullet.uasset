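; Bullet projectile Blueprint that damages what it strikes and spawns a dust explosion when destroyed.
; While activated, both hit and overlap events feed one handler that ignores its owner and objects of its own class.
; The handler sends damage through the BPI_Damageable interface, notifies a BP_Striker owner when a damageable target is struck, then destroys the bullet.
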(event `self.ReceiveDestroyed`
  (`GameplayStatics.SpawnEmitterAtLocation` "/Game/Strikers/Particles/P_DustExplosion.P_DustExplosion" (`SceneComponent.K2_GetComponentLocation` (`self.Capsule`))))

(event `self.ReceiveHit`
  (params (MyComp :type "PrimitiveComponent Object Reference") (Other :type "Actor Object Reference") (OtherComp :type "PrimitiveComponent Object Reference") (bSelfMoved :type Boolean) (HitLocation :type "Vector Structure") (HitNormal :type "Vector Structure") (NormalImpulse :type "Vector Structure") (Hit :type "HitResult Structure (by ref)"))
  (if (`self.IsActivated`)
    (`self.HitSomething` Other)))

(event `self.ReceiveActorBeginOverlap`
  (params (OtherActor :type "Actor Object Reference"))
  (if (`self.IsActivated`)
    (`self.HitSomething` OtherActor)))

(event `HitSomething`
  (params (Something :type "Actor Object Reference"))
  (bind _returnvalue (`KismetSystemLibrary.DoesImplementInterface` Something "/Game/Strikers/Blueprints/BPI_Damageable.BPI_Damageable_C"))
  (if (and (!= (`GameplayStatics.GetObjectClass` Something) (`GameplayStatics.GetObjectClass` self)) (!= Something (`self.ProjectileOwner`)))
    (if _returnvalue
      (message `/Game/Strikers/Blueprints/BPI_Damageable.TakeDamage` Something (`self.Damage`) (`self.ProjectileOwner`)))
    (`/Engine/EditorBlueprintResources/StandardMacros.IsValid` (`self.ProjectileOwner`)
      (:`Is Valid`
        (if _returnvalue
          (bind _asbp_striker (cast `/Game/Strikers/Blueprints/FlyingCharacter/BP_Striker` (`self.ProjectileOwner`))
            (:`then`
              (`/Game/Strikers/Blueprints/FlyingCharacter/BP_Striker.DamagedSomething` _asbp_striker))
            (:`CastFailed`
              _))))
      (:`Is Not Valid`
        _))
    (`self.K2_DestroyActor`)))

(fn `UserConstructionScript`
  (`parent.UserConstructionScript`))