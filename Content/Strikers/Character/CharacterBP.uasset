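; CharacterBP is a Strikers character Blueprint that turns axis inputs into camera-relative movement and controller rotation.
; MoveForward adds movement along the Camera's full forward vector, vertical component included.
; Turn drives controller yaw, MoveRoll drives roll, and both LookUp and MovePitch drive pitch.
; It has no other active logic: BeginPlay, overlap and Tick are disabled, and the construction script is empty.
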(event `InputAxis|Turn`
  (params (AxisValue :type "Float (single-precision)"))
  (`self.AddControllerYawInput` AxisValue))

(event `InputAxis|LookUp`
  (params (AxisValue :type "Float (single-precision)"))
  (`self.AddControllerPitchInput` AxisValue))

(event `InputAxis|MoveForward`
  (params (AxisValue :type "Float (single-precision)"))
  (bind (_returnvalue_x _returnvalue_y _returnvalue_z) (`KismetMathLibrary.BreakVector` (`SceneComponent.GetForwardVector` (`self.Camera`))))
  (`self.AddMovementInput` (`KismetMathLibrary.MakeVector` _returnvalue_x _returnvalue_y _returnvalue_z) AxisValue))

(event `InputAxis|MoveRoll`
  (params (AxisValue :type "Float (single-precision)"))
  (`self.AddControllerRollInput` AxisValue))

(event `InputAxis|MovePitch`
  (params (AxisValue :type "Float (single-precision)"))
  (`self.AddControllerPitchInput` AxisValue))

(fn `UserConstructionScript`)